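; BP_Player is a first-person player pawn that moves, looks around and fires a rifle.
; Axis inputs drive movement along the actor's forward and right vectors, plus controller yaw and pitch.
; On BeginPlay it spawns a BP_Rifle, stores it as EquippedGun and snaps it to GunLocation.
; While the Shoot axis truncates to 1, it calls the gun's Shoot from FpsCamera along its forward vector to the gun's maximum bullet distance.
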(event `InputAxis|MoveFoward`
  (params (AxisValue :type "Float (single-precision)"))
  (`self.AddMovementInput` (`self.GetActorForwardVector`) AxisValue))

(event `InputAxis|MoveRight`
  (params (AxisValue :type "Float (single-precision)"))
  (`self.AddMovementInput` (`self.GetActorRightVector`) AxisValue))

(event `InputAxis|LookHorizontal`
  (params (AxisValue :type "Float (single-precision)"))
  (`self.AddControllerYawInput` AxisValue))

(event `InputAxis|LookVertical`
  (params (AxisValue :type "Float (single-precision)"))
  (`self.AddControllerPitchInput` AxisValue))

(event `self.ReceiveBeginPlay`
  (bind _returnvalue (`|SpawnActorFromClass` "/Game/Blueprints/BP_Rifle.BP_Rifle_C" (`KismetMathLibrary.MakeTransform` (0.0 0.0 0.0)) "Undefined" "OverrideRootScale" null null))
  (bind _output_get (set `self.EquippedGun` _returnvalue))
  (`self.K2_AttachToComponent` _output_get (`self.GunLocation`) "None" "SnapToTarget" "SnapToTarget" "KeepRelative" true))

(event `InputAxis|Shoot`
  (params (AxisValue :type "Float (single-precision)"))
  (bind _fpscamera (`self.FpsCamera`))
  (bind _returnvalue (`SceneComponent.K2_GetComponentLocation` _fpscamera))
  (if (== (`KismetMathLibrary.FTrunc` AxisValue) 1)
    (`/Game/Blueprints/BP_BaseGun.Shoot` (`self.EquippedGun`) _returnvalue (+ _returnvalue (* (`SceneComponent.GetForwardVector` _fpscamera) (`/Game/Blueprints/BP_BaseGun.MaxBulletDistance` (`self.EquippedGun`)))))))

(fn `UserConstructionScript`)